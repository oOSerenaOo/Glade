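; BPC_Inventory is a player component that currently handles interacting with actors in front of the first-person character.
; It caches the character on BeginPlay; on IA_Interact it sphere-traces a short distance from the camera along control rotation, with debug drawing.
; A hit actor receives BPIInteractMessage, leaving the response to that actor.
; Tag-based Axe and Log pickup logic is disconnected, and the trace's ImpactPoint output actually carries the impact normal.
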(event Input|EnhancedActionEvents|EnhancedInputActionIA_Interact
  (params (ActionValue :type Boolean) (ElapsedSeconds :type Float%20%28double-precision%29) (TriggeredSeconds :type Float%20%28double-precision%29) (InputAction :type Input%20Action%20Object%20Reference :default "/Game/FirstPerson/Input/Actions/IA_Interact.IA_Interact"))
  ;[1 1 1] Interact
  (:Started
    (bind (_hitactor _actorhit_) (CallFunction|InteractSphereTrace))
    (if _actorhit_
      (Class|BPIInteract|BPIInteract(Message) _hitactor))))

(event EventBeginPlay
  (bind _asbp_first_person_character (Utilities|Casting|CastToBP_FirstPersonCharacter (Game|Player|GetPlayerPawn 0)))
  (Variables|Default|SetFirst%20Person%20Character _asbp_first_person_character))

(event EventTick
  (params (DeltaSeconds :type Float%20%28single-precision%29)))

(fn InteractSphereTrace
  (bind _first_person_character (Variables|Default|GetFirst%20Person%20Character))
  (bind _firstpersoncamera (Variables|/Game/FirstPerson/Blueprints/BP_FirstPersonCharacter.BP_FirstPersonCharacter_C|GetFirstPersonCamera _first_person_character))
  (bind _returnvalue (Transformation|GetWorldLocation _firstpersoncamera))
  (bind (_outhit _returnvalue_2) (Collision|SphereTraceByChannel _returnvalue (+ _returnvalue (* (Math|Vector|GetForwardVector (Pawn|GetControlRotation _first_person_character :!class /Script/Engine.Pawn)) 3e+02)) 2e+01 "TraceTypeQuery1" false 0 "ForDuration" true "(R=1.000000,G=0.000000,B=0.000000,A=1.000000)" "(R=0.000000,G=1.000000,B=0.000000,A=1.000000)" 2.0))
  (if _returnvalue_2
    (return (.HitActor (Collision|BreakHitResult _outhit)) true (.ImpactNormal (Collision|BreakHitResult _outhit)))
    (else
      (return 0 false (.ImpactNormal (Collision|BreakHitResult _outhit))))))